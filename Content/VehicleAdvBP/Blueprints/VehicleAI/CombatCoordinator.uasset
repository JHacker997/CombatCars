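; CombatCoordinator picks steering behaviors for AI vehicle followers in combat.
; Tick accumulates a single timer; when DecideState finds it past the follower's StateTime, it resets it and randomly chooses Seek, Pursue, Flee or Wander, with the range read from the EnemyValues data table.
; Targeted behaviors always use player pawn 0.
; GetClosestPlayer is unfinished: its distance comparison is disconnected, so the multi-vehicle branch returns no selected vehicle.
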(event `self.ReceiveTick`
  (params (DeltaSeconds :type "Float (single-precision)"))
  (set `self.Counter` (+ DeltaSeconds (`self.Counter`))))

(fn `DecideState`
  (params (Follower :type "/Game/VehicleAdvBP/Blueprints/VehicleAI/Follower Object Reference"))
  (bind _returnvalue (`GameplayStatics.GetPlayerPawn` 0))
  (if (>= (`self.Counter`) (`/Game/VehicleAdvBP/Blueprints/VehicleAI/Follower.StateTime` Follower))
    (set `self.Counter` 0.0)
    (bind _returnvalue_2 (`|GetDataTableRow` (`self.EnemyValues`) (`self.StatesAmountName`))
      (:`then`
        (switch `int` (`KismetMathLibrary.RandomIntegerInRange` 0 (- (`.Value_2_B2300F7E45EF0B4B495D8597826E13CA` (break `/Game/VehicleAdvBP/Blueprints/DataDrivenValues/GameData` _returnvalue_2)) 1))
          (:`Default`
            (`/Game/VehicleAdvBP/Blueprints/VehicleAI/Follower.Seek` Follower _returnvalue :!label _label))
          (:`0`
            (goto _label))
          (:`1`
            (`/Game/VehicleAdvBP/Blueprints/VehicleAI/Follower.Pursue` Follower _returnvalue))
          (:`2`
            (`/Game/VehicleAdvBP/Blueprints/VehicleAI/Follower.Flee` Follower _returnvalue))
          (:`3`
            (`/Game/VehicleAdvBP/Blueprints/VehicleAI/Follower.Wander` Follower)))))))

(fn `GetClosestPlayer`
  (params (Follower :type "/Game/VehicleAdvBP/Blueprints/VehicleAI/Follower Object Reference"))
  (returns (Player :type "/Game/VehicleAdvBP/Blueprints/VehicleAI/VehicleBlueprint Object Reference"))
  (bind _asvehicle_blueprint (cast `/Game/VehicleAdvBP/Blueprints/VehicleAI/VehicleBlueprint` (`GameplayStatics.GetPlayerPawn` 0)))
  (if (== (`KismetArrayLibrary.Array_Length` (stale _outactors)) 1)
    (return _asvehicle_blueprint)
    (else
      (bind _outactors (`GameplayStatics.GetAllActorsOfClass` (`GameplayStatics.GetObjectClass` _asvehicle_blueprint)))
      (for (_array_element _array_index) _outactors
        (bind _returnvalue (`KismetMathLibrary.VSize` (- (`Actor.K2_GetActorLocation` Follower) (`Actor.K2_GetActorLocation` _array_element))))
        (bind _array (`|MakeArray` _returnvalue))
        (`KismetArrayLibrary.Array_Set` _array _array_index _returnvalue true))
      (for (_array_element_2 _array_index_2) _array
        _))))