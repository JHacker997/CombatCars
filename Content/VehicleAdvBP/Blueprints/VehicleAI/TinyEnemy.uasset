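; TinyEnemy is a small enemy variant in the vehicle AI, extending a parent Blueprint that supplies its base behavior.
; On BeginPlay it runs the parent logic, then sets MaxSpeed from the TinySpeed row of the EnemyValues data table.
; A DoOnce on Tick, after the parent tick, calls SwapGuns on the GunController a single time to switch its weapon.
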(event `self.ReceiveBeginPlay`
  (`parent.ReceiveBeginPlay`)
  (bind _returnvalue (`|GetDataTableRow` "/Game/VehicleAdvBP/Blueprints/DataDrivenValues/EnemyValues.EnemyValues" "TinySpeed")
    (:`then`
      (set `self.MaxSpeed` (`KismetMathLibrary.Conv_IntToDouble` (`.Value_2_B2300F7E45EF0B4B495D8597826E13CA` (break `/Game/VehicleAdvBP/Blueprints/DataDrivenValues/GameData` _returnvalue)))))))

(event `self.ReceiveTick`
  (params (DeltaSeconds :type "Float (single-precision)"))
  (`parent.ReceiveTick` DeltaSeconds)
  (`/Engine/EditorBlueprintResources/StandardMacros.DoOnce` false
    (:`Completed`
      (`GunController.swapGuns` (`self.GunController`)))))

(fn `UserConstructionScript`
  (`parent.UserConstructionScript`))