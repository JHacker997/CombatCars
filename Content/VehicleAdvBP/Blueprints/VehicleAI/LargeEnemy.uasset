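; LargeEnemy is a vehicle AI Blueprint for the large enemy type, extending a parent enemy class.
; On BeginPlay it runs the parent logic, then reads its speed row from the EnemyValues data table and stores it as MaxSpeed.
; Overlap and Tick events are disabled, and construction only calls the parent, so the remaining behavior comes from the parent.
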(event `self.ReceiveBeginPlay`
  (`parent.ReceiveBeginPlay`)
  (bind _returnvalue (`|GetDataTableRow` (`self.EnemyValues`) (`self.LargeSpeedName`))
    (:`then`
      (set `self.MaxSpeed` (`KismetMathLibrary.Conv_IntToDouble` (`.Value_2_B2300F7E45EF0B4B495D8597826E13CA` (break `/Game/VehicleAdvBP/Blueprints/DataDrivenValues/GameData` _returnvalue)))))))

(fn `UserConstructionScript`
  (`parent.UserConstructionScript`))