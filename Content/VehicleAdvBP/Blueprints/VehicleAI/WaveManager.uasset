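; Wave manager that runs nine waves of small and large AI followers, then calls VICTORY on the player vehicle.
; BeginPlay loads per-wave counts from a data table.
; DecideSpawn uses random spawners (small waves draw from SpawnerLarge, large from SpawnerSmall), re-arming a timer until counts are met.
; Tick periodically prunes invalid small-wave entries and advances once both fully spawned lists empty; RemoveActor removes followers from both.
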(event `self.ReceiveBeginPlay`
  (for _index (range 9)
    (bind _returnvalue (`|GetDataTableRow` "/Game/VehicleAdvBP/Blueprints/DataDrivenValues/Testing_-_Sheet1.Testing_-_Sheet1" (`KismetStringLibrary.Conv_StringToName` (`KismetStringLibrary.Conv_IntToString` _index)))
      (:`then`
        (bind (_smallenemies _largeenemies) (break `/Game/VehicleAdvBP/Blueprints/DataDrivenValues/WaveData` _returnvalue))
        (`KismetArrayLibrary.Array_Set` (`self.Small Wave Size`) _index _smallenemies true)
        (`KismetArrayLibrary.Array_Set` (`self.Large Wave Size`) _index _largeenemies true)))))

(event `self.ReceiveTick`
  (params (DeltaSeconds :type "Float (single-precision)"))
  (bind _timedealy (`self.TimeDealy`))
  (bind _wavenumber (`self.WaveNumber`))
  (if (< _timedealy 5.0)
    (set `self.TimeDealy` (+ DeltaSeconds _timedealy))
    (else
      (set `self.TimeDealy` 0.0)
      (`self.CleanWave`)
      (if (and (<= (`KismetArrayLibrary.Array_Length` (`self.CurrentSmallWave`)) 0) (<= (`KismetArrayLibrary.Array_Length` (`self.CurrentLargeWave`)) 0) (== (`self.CurrSmallWaveSize`) (`|GetArrayItem` (`self.Small Wave Size`) (`self.WaveNumber`))) (== (`self.CurrLargeWaveSize`) (`|GetArrayItem` (`self.Large Wave Size`) (`self.WaveNumber`))))
        (set `self.CurrSmallWaveSize` 0)
        (set `self.CurrLargeWaveSize` 0)
        (`/Engine/EditorBlueprintResources/StandardMacros.IncrementInt` _wavenumber
          (:`  `
            (if (< _wavenumber 9)
              (`self.DecideSpawn`)
              (else
                (bind _outactors (`GameplayStatics.GetAllActorsOfClass` "/Game/VehicleAdvBP/Blueprints/VehicleAI/VehicleBlueprint.VehicleBlueprint_C"))
                (`/Game/VehicleAdvBP/Blueprints/VehicleAI/VehicleBlueprint.VICTORY` (`|GetArrayItem` _outactors))))))))))

(fn `CleanWave`
  (for (_array_element _array_index) (`self.CurrentSmallWave`)
    (`/Engine/EditorBlueprintResources/StandardMacros.IsValid` _array_element
      (:`Is Not Valid`
        (`KismetArrayLibrary.Array_Remove` (`self.CurrentSmallWave`) _array_index)))))

(fn `DecideSpawn`
  (bind _spawnersmall (`self.SpawnerSmall`))
  (bind _spawnerlarge (`self.SpawnerLarge`))
  (bind _returnvalue (< (`self.CurrLargeWaveSize`) (`|GetArrayItem` (`self.Large Wave Size`) (`self.WaveNumber`))))
  (bind _returnvalue_2 (< (`self.CurrSmallWaveSize`) (`|GetArrayItem` (`self.Small Wave Size`) (`self.WaveNumber`))))
  (`|ExecutionSequence`
    (:`then_0`
      (if _returnvalue_2
        (bind _spawnedfollower (`/Game/VehicleAdvBP/Blueprints/VehicleAI/EnemySpawner.Spawn` (`|GetArrayItem` _spawnerlarge (`KismetMathLibrary.RandomInteger` (`KismetArrayLibrary.Array_Length` _spawnerlarge)))))
        (bind _returnvalue_3 (`KismetArrayLibrary.Array_Add` (`self.CurrentSmallWave`) _spawnedfollower))
        (set `/Game/VehicleAdvBP/Blueprints/VehicleAI/Follower.ManagerIndex` _returnvalue_3 _spawnedfollower)
        (`/Engine/EditorBlueprintResources/StandardMacros.IncrementInt` (`self.CurrSmallWaveSize`)
          (:`  `
            (if _returnvalue_2
              (`KismetSystemLibrary.K2_SetTimer` self "DecideSpawn" 5.0))))))
    (:`then_1`
      (if _returnvalue
        (bind _spawnedfollower_2 (`/Game/VehicleAdvBP/Blueprints/VehicleAI/EnemySpawner.Spawn` (`|GetArrayItem` _spawnersmall (`KismetMathLibrary.RandomInteger` (`KismetArrayLibrary.Array_Length` _spawnersmall)))))
        (bind _returnvalue_4 (`KismetArrayLibrary.Array_Add` (`self.CurrentLargeWave`) _spawnedfollower_2))
        (set `/Game/VehicleAdvBP/Blueprints/VehicleAI/Follower.ManagerIndex` _returnvalue_4 _spawnedfollower_2)
        (`/Engine/EditorBlueprintResources/StandardMacros.IncrementInt` (`self.CurrLargeWaveSize`)
          (:`  `
            (if _returnvalue
              (`KismetSystemLibrary.K2_SetTimer` self "DecideSpawn" 5.0))))))))

(fn `RemoveActor`
  (params (ActorToRemove :type "/Game/VehicleAdvBP/Blueprints/VehicleAI/Follower Object Reference") (Index :type Integer))
  (`KismetArrayLibrary.Array_RemoveItem` (`self.CurrentSmallWave`) ActorToRemove)
  (`KismetArrayLibrary.Array_RemoveItem` (`self.CurrentLargeWave`) ActorToRemove))

(fn `UserConstructionScript`)