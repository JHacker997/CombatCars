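; Boss actor in the vehicle AI folder that carries turret child actors and turns one toward a referenced actor, NewVar0.
; Each Tick sets Turret2Blueprint's world yaw from the acos of the 2D dot product of both normalized world positions, keeping the boss's roll and pitch.
; That angle is unsigned and measured about the world origin, not along the turret-to-target direction.
; A relative-rotation variant and a three-turret Fire chain are unconnected, so the boss never fires here.
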(event `self.ReceiveTick`
  (params (DeltaSeconds :type "Float (single-precision)"))
  (`SceneComponent.K2_SetWorldRotation` (`self.Turret2Blueprint`) (`KismetMathLibrary.MakeRotator` (.roll (.rotation (`self.GetTransform`))) (.pitch (.rotation (`self.GetTransform`))) (* (`KismetMathLibrary.DegAcos` (`KismetMathLibrary.DotProduct2D` (`KismetMathLibrary.Normal2D` (`KismetMathLibrary.Conv_VectorToVector2D` (`self.K2_GetActorLocation` (`self.NewVar_0`)))) (`KismetMathLibrary.Normal2D` (`KismetMathLibrary.Conv_VectorToVector2D` (`self.K2_GetActorLocation` (`ChildActorComponent.ChildActor` (`self.Turret2Blueprint`))))))) 1.0)) false false))

(fn `UserConstructionScript`)