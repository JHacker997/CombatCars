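; Powerup pickup actor for vehicles that is consumed on overlap and triggers its spawner to respawn it.
; Any overlapping actor not tagged Bullet destroys the pickup, but only a VehicleBlueprint tagged Player receives the Powerup call.
; On destruction it casts its owner to PickUpSpawner and calls SpawnOnDelay, leaving respawn timing to the spawner.
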(event `self.ReceiveActorBeginOverlap`
  (params (OtherActor :type "Actor Object Reference"))
  (if (not (`self.ActorHasTag` OtherActor "Bullet"))
    (`self.K2_DestroyActor`)
    (if (`self.ActorHasTag` OtherActor "Player")
      (bind _asvehicle_blueprint (cast `/Game/VehicleAdvBP/Blueprints/VehicleAI/VehicleBlueprint` OtherActor))
      (`/Game/VehicleAdvBP/Blueprints/VehicleAI/VehicleBlueprint.Powerup` _asvehicle_blueprint))))

(event `self.ReceiveDestroyed`
  (bind _aspick_up_spawner (cast `/Game/VehicleAdvBP/Blueprints/Powerups/PickUpSpawner` (`self.GetOwner`)))
  (`/Game/VehicleAdvBP/Blueprints/Powerups/PickUpSpawner.SpawnOnDelay` _aspick_up_spawner))

(fn `UserConstructionScript`)