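; BulletBlueprint is a projectile that damages opposing actors on hit and destroys itself on contact with anything not tagged Pickup.
; Actor tags on its owner and target separate Player from Enemy and mark what is Damageable.
; The target's DamageController applies fixed damage and returns health, which is copied to a VehicleBlueprint target.
; At zero health the target is destroyed, triggering game over for a vehicle or otherwise awarding score to a vehicle owner.
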(event `self.ReceiveHit`
  (params (MyComp :type "PrimitiveComponent Object Reference") (Other :type "Actor Object Reference") (OtherComp :type "PrimitiveComponent Object Reference") (bSelfMoved :type Boolean) (HitLocation :type "Vector Structure") (HitNormal :type "Vector Structure") (NormalImpulse :type "Vector Structure") (Hit :type "HitResult Structure (by ref)"))
  (bind _returnvalue (`self.GetOwner`))
  ;[1 1 1] If the Bullet is currently pending kill then ignore
  (if (not (`self.IsActorBeingDestroyed`))
    ;[1 1 1] If its a pickup we ignore it and dont destroy ourself
    (if (not (`self.ActorHasTag` Other "Pickup"))
      ;[1 1 1] If we are on oppositeTeams
      (if (or (and (`self.ActorHasTag` _returnvalue "Enemy") (`self.ActorHasTag` Other "Player")) (and (`self.ActorHasTag` Other "Enemy") (`self.ActorHasTag` _returnvalue "Player")))
        ;[1 1 1] And it can be damaged
        (if (`self.ActorHasTag` Other "Damageable")
          ;[1 1 1] Apply damage using its Damage controller
          (bind _returnvalue_2 (`DamageController.ApplyDamage` (`self.GetComponentByClass` Other "/Script/CombatCars2.DamageController") 10))
          ;[1 1 1] If it is a VBP thenset health
          (bind _asvehicle_blueprint (cast `/Game/VehicleAdvBP/Blueprints/VehicleBlueprint` Other)
            (:`then`
              (set `/Game/VehicleAdvBP/Blueprints/VehicleBlueprint.Health` _returnvalue_2 _asvehicle_blueprint))
            (:`CastFailed`
              _))
          ;[1 1 1] If we set their Health to 0, destroy them
          (if (== _returnvalue_2 0.0)
            ;;[1 1 1] And if its the player then they lose
            (bind _asvehicle_blueprint_2 (cast `/Game/VehicleAdvBP/Blueprints/VehicleBlueprint` Other)
              (:`then`
                (`/Game/VehicleAdvBP/Blueprints/VehicleBlueprint.GAMEOVER` _asvehicle_blueprint_2))
              (:`CastFailed`
                ;;[1 1 1] Otherwise, if Im owned by the player increase score
                (bind _asvehicle_blueprint_3 (cast `/Game/VehicleAdvBP/Blueprints/VehicleBlueprint` (`self.GetOwner`))
                  (:`then`
                    (`/Game/VehicleAdvBP/Blueprints/VehicleBlueprint.ChangeScore` _asvehicle_blueprint_3 100))
                  (:`CastFailed`
                    _))))
            (`self.K2_DestroyActor` Other))))
      ;[1 1 1] Otherwise, just destroy us
      (`self.K2_DestroyActor`))))

(fn `UserConstructionScript`)