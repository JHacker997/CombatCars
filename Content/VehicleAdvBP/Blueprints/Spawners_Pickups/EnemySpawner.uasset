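; Enemy spawner that creates an actor of a configurable type at its own transform, on BeginPlay and on a looping timer.
; Each Spawn call is skipped while the referenced SpawnedTarget is flagged Invincible.
; It calls SpawnDefaultController on the new actor's Instigator.
; If the actor is a Follower, it sets max health from SpawnHealth and calls KillChildren on its GunController.
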(event `self.ReceiveBeginPlay`
  (`self.Spawn`)
  (`KismetSystemLibrary.K2_SetTimer` null "Spawn" 10.0 true))

(fn `Spawn`
  (set `self.Spawning?` (`/Game/VehicleAdvBP/Blueprints/VehicleBlueprint.invincible` (`self.Spawned Target`)))
  (if (not (`self.Spawning?`))
    (bind _returnvalue (`|SpawnActorFromClass` (`self.SpawnType`) (`self.GetTransform`) "Undefined" "OverrideRootScale" null null))
    (`Pawn.SpawnDefaultController` (`Actor.Instigator` _returnvalue))
    (bind _asfollower (cast `/Game/VehicleAdvBP/Blueprints/Follower` _returnvalue))
    (`DamageController.SetHealthMax` (`/Game/VehicleAdvBP/Blueprints/Follower.DamageController` _asfollower) (`self.Spawn Health`))
    (`GunController.killChildren` (`/Game/VehicleAdvBP/Blueprints/Follower.GunController` _asfollower))))

(fn `UserConstructionScript`)