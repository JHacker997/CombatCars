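; EnemySpawner is an actor that can spawn a TinyEnemy vehicle at its own transform through its Spawn function.
; Spawn gives the enemy a default controller, sets its max health to 100, calls KillChildren on its gun controller and activates vehicle movement.
; Nothing in the file triggers Spawn: the direct call and looping timer are unwired, as is the assignment of SpawnedTarget as target and waypoint.
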(event `self.ReceiveBeginPlay`)

(fn `Spawn`
  (bind _returnvalue (`|SpawnActorFromClass` "/Game/VehicleAdvBP/Blueprints/TinyEnemy.TinyEnemy_C" (`self.GetTransform`) "Undefined" "OverrideRootScale" null null))
  (`Pawn.SpawnDefaultController` _returnvalue)
  (`DamageController.SetHealthMax` (`/Game/VehicleAdvBP/Blueprints/Follower.DamageController` _returnvalue) 100)
  (`GunController.killChildren` (`/Game/VehicleAdvBP/Blueprints/Follower.GunController` _returnvalue))
  (`ActorComponent.Activate` (`WheeledVehicle.VehicleMovement` _returnvalue) false))

(fn `UserConstructionScript`)