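; Turret bullet that damages actors on the opposing Player or Enemy team and destroys itself on hitting anything but a pickup.
; On BeginPlay it reads Damage from the PlayerValues table and, if the row is found, ignores pickups while moving.
; Hits apply damage through the target's DamageController, updating vehicle health.
; Kills trigger a larger explosion, plus game over for a vehicle or score for a vehicle owner otherwise.
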(event `self.ReceiveHit`
  (params (MyComp :type "PrimitiveComponent Object Reference") (Other :type "Actor Object Reference") (OtherComp :type "PrimitiveComponent Object Reference") (bSelfMoved :type Boolean) (HitLocation :type "Vector Structure") (HitNormal :type "Vector Structure") (NormalImpulse :type "Vector Structure") (Hit :type "HitResult Structure (by ref)"))
  (bind _returnvalue (`self.GetOwner`))
  (bind _explosionmultiplier (`self.ExplosionMultiplier`))
  (bind _explosionmultiplier_2 (`self.ExplosionMultiplier`))
  (bind _returnvalue_2 (or (and (`self.ActorHasTag` _returnvalue "Enemy") (`self.ActorHasTag` Other "Player")) (and (`self.ActorHasTag` Other "Enemy") (`self.ActorHasTag` _returnvalue "Player"))))
  ;[1 1 1] If the Bullet is currently pending kill then ignore
  (if (not (`self.IsActorBeingDestroyed`))
    ;[1 1 1] Is tagert currently being destroyed
    (if (not (`self.IsActorBeingDestroyed` Other))
      ;[1 1 1] If its a pickup we ignore it and dont destroy ourself
      (if (not (`self.ActorHasTag` Other "Pickup"))
        ;[1 1 1] Check if it is a wall and ignore
        (if (`self.ActorHasTag` Other "Wall")
          _
          (else
            _))
        ;[1 1 1] If we are on oppositeTeams
        (if _returnvalue_2
          ;[1 1 1] And it can be damaged
          (if (`self.ActorHasTag` Other "Damageable")
            ;[1 1 1] Apply damage using its Damage controller
            (bind _returnvalue_3 (`DamageController.ApplyDamage` (`self.GetComponentByClass` Other "/Script/CombatCars2.DamageController") (`self.Damage`)))
            ;[1 1 1] If it is a VBP thenset health
            (bind _asvehicle_blueprint (cast `/Game/VehicleAdvBP/Blueprints/VehicleAI/VehicleBlueprint` Other)
              (:`then`
                (set `/Game/VehicleAdvBP/Blueprints/VehicleAI/VehicleBlueprint.Health` _returnvalue_3 _asvehicle_blueprint))
              (:`CastFailed`
                _))
            ;[1 1 1] If we set their Health to 0, destroy them
            (if (== _returnvalue_3 0.0)
              ;;[1 1 1] And if its the player then they lose
              (bind _asvehicle_blueprint_2 (cast `/Game/VehicleAdvBP/Blueprints/VehicleAI/VehicleBlueprint` Other)
                (:`then`
                  (`/Game/VehicleAdvBP/Blueprints/VehicleAI/VehicleBlueprint.GAMEOVER` _asvehicle_blueprint_2))
                (:`CastFailed`
                  ;;[1 1 1] Otherwise, if Im owned by the player increase score
                  (bind _asvehicle_blueprint_3 (cast `/Game/VehicleAdvBP/Blueprints/VehicleAI/VehicleBlueprint` (`self.GetOwner`))
                    (:`then`
                      (`/Game/VehicleAdvBP/Blueprints/VehicleAI/VehicleBlueprint.ChangeScore` _asvehicle_blueprint_3 100))
                    (:`CastFailed`
                      _))))
              (`self.K2_DestroyActor` Other)
              ;[1 1 1] Explosion particle and sound effects
              (bind _returnvalue_4 (`GameplayStatics.SpawnEmitterAtLocation` "/Game/StarterContent/Particles/P_Explosion.P_Explosion" (`SceneComponent.K2_GetComponentLocation` (`self.Bullet`)) (struct) (* (`KismetMathLibrary.MakeVector` _explosionmultiplier _explosionmultiplier _explosionmultiplier) 3.0)))
              (`GameplayStatics.SpawnSoundAttached` "/Game/StarterContent/Audio/Explosion02.Explosion02" _returnvalue_4))))
        (if _returnvalue_2
          (`|ExecutionSequence`
            (:`then_0`
              (`/Engine/EditorBlueprintResources/StandardMacros.DoOnce` false
                (:`Completed`
                  (bind _returnvalue_5 (`GameplayStatics.SpawnEmitterAtLocation` "/Game/StarterContent/Particles/P_Explosion.P_Explosion" (`SceneComponent.K2_GetComponentLocation` (`self.Bullet`)) (struct) (`KismetMathLibrary.MakeVector` _explosionmultiplier_2 _explosionmultiplier_2 _explosionmultiplier_2)))
                  (`GameplayStatics.SpawnSoundAttached` "/Game/StarterContent/Audio/Explosion01.Explosion01" _returnvalue_5 "None" (0.0 0.0 0.0) (struct) "KeepRelativeOffset" false 0.5))))
            (:`then_1`
              ;;[1 1 1] Destroy the bullet
              (`self.K2_DestroyActor` :!label _label)))
          (else
            (goto _label)))))))

(event `self.ReceiveBeginPlay`
  (bind _returnvalue (`|GetDataTableRow` (`self.PlayerValues`) (`self.RedBulletDamageName`))
    (:`then`
      (set `self.Damage` (`.Value_2_B2300F7E45EF0B4B495D8597826E13CA` (break `/Game/VehicleAdvBP/Blueprints/DataDrivenValues/GameData` _returnvalue)))
      (bind _outactors (`GameplayStatics.GetAllActorsWithTag` "Pickup"))
      (for _array_element _outactors
        (`PrimitiveComponent.IgnoreActorWhenMoving` (`self.Bullet`) _array_element true)))))

(fn `UserConstructionScript`)