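; Turret actor in the VehicleAdvBP vehicle project that fires bullets on demand through its Fire function.
; Fire spawns a scaled-down BulletBlueprint at the Scene component's world location and rotation, with the passed Shooter as owner.
; The RelativeTransform input has no effect on the spawn, as it feeds only disconnected offset math left in the graph.
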(fn `Fire`
  (params (Shooter :type "Actor Object Reference") (RelativeTransform :type "Vector Structure"))
  (bind _scene (`self.Scene`))
  (`|SpawnActorFromClass` "/Game/VehicleAdvBP/Blueprints/Turrets/BulletBlueprint.BulletBlueprint_C" (`KismetMathLibrary.MakeTransform` (`SceneComponent.K2_GetComponentLocation` _scene) (`SceneComponent.K2_GetComponentRotation` _scene) (0.05 0.1 0.05)) "Undefined" "OverrideRootScale" Shooter null))

(fn `UserConstructionScript`)